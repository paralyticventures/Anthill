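; Test boss enemy character built on the Gameplay Ability System, with a health bar, melee attack and ragdoll death.
; Attribute-change listeners reveal the initially hidden bar when the value drops below a reference attribute and trigger death at zero.
; Death plays a sound, detaches the controller, ragdolls the mesh and delays actor destruction.
; Damage snaps it toward the causer, while DoMeleeHit sphere-traces forward with debug drawing and applies GE_BossHit.
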(event `self.ReceiveBeginPlay`
  (bind _returnvalue (`|CreateWidget` "/Game/Blueprints/Widgets/WBP_EnemyHealthBar.WBP_EnemyHealthBar_C" null self))
  (`WidgetComponent.SetWidget` (`self.Widget`) _returnvalue)
  (`SceneComponent.SetVisibility` (`self.Widget`) false false)
  (bind (_asynctaskproxy _attribute _newvalue) (`AbilityAsync_WaitAttributeChanged.WaitForAttributeChanged` null (struct :`AttributeName` "Health" :`Attribute` "/Script/Anthill.BasicAttributeSet:Health" :`AttributeOwner` "/Script/CoreUObject.Class'/Script/Anthill.BasicAttributeSet'"))
    (:`then`
      (bind (_asynctaskproxy_2 _attribute_2 _newvalue_2) (`AbilityAsync_WaitAttributeChanged.WaitForAttributeChanged` null (struct :`AttributeName` "Health" :`Attribute` "/Script/Anthill.BasicAttributeSet:Health" :`AttributeOwner` "/Script/CoreUObject.Class'/Script/Anthill.BasicAttributeSet'"))
        (:`Changed`
          (if (< _newvalue_2 (`.ReturnValue` (`AbilitySystemBlueprintLibrary.GetFloatAttributeFromAbilitySystemComponent` (`self.AbilitySystemComponent`) (struct :`AttributeName` "MaxHealth" :`Attribute` "/Script/Anthill.BasicAttributeSet:MaxHealth" :`AttributeOwner` "/Script/CoreUObject.Class'/Script/Anthill.BasicAttributeSet'"))))
            (bind _widget (`self.Widget`)
              (:`then`
                (`SceneComponent.SetVisibility` _widget true false))
              (:`else`))))))
    (:`Changed`
      (if (<= _newvalue 0.0)
        (`self.Die`)))))

(event `Die`
  (bind _mesh (`self.Mesh`))
  (`GameplayStatics.PlaySoundAtLocation` "/Game/Audio/BossDeathSound.BossDeathSound" (`self.K2_GetActorLocation` self) (struct) 1.0 1.0 0.0 null null null null)
  (`self.DetachFromControllerPendingDestroy`)
  (`ActorComponent.Deactivate` (`self.CharacterMovement`))
  (`PrimitiveComponent.SetCollisionEnabled` (`self.CapsuleComponent`) "NoCollision")
  (`PrimitiveComponent.SetCollisionProfileName` _mesh "Ragdoll" true)
  (`SkeletalMeshComponent.SetAllBodiesSimulatePhysics` _mesh true)
  (`PrimitiveComponent.WakeAllRigidBodies` _mesh)
  (`SkeletalMeshComponent.SetAnimInstanceClass` _mesh null)
  (bind _widget (`self.Widget`)
    (:`then`
      (`ActorComponent.K2_DestroyComponent` _widget)
      (set `self.Dead` true)
      (`KismetSystemLibrary.Delay` 20.0)
      (`self.K2_DestroyActor`))
    (:`else`)))

(event `self.ReceiveAnyDamage`
  (params (Damage :type "Float (single-precision)") (DamageType :type "DamageType Object Reference") (InstigatedBy :type "Controller Object Reference") (DamageCauser :type "Actor Object Reference"))
  (`self.K2_SetActorRotation` (`KismetMathLibrary.FindLookAtRotation` (`self.K2_GetActorLocation`) (`self.K2_GetActorLocation` DamageCauser))))

(fn `DoMeleeHit`
  (bind _outhit (`KismetSystemLibrary.SphereTraceSingle` :`Start` (`self.K2_GetActorLocation`) :`End` (+ (`self.K2_GetActorLocation`) (* (`KismetMathLibrary.GetForwardVector` (`self.GetControlRotation`)) 150.0)) :`Radius` 100.0 :`TraceChannel` "TraceTypeQuery1" :`bTraceComplex` true :`DrawDebugType` "ForDuration"))
  (`AbilitySystemComponent.BP_ApplyGameplayEffectToTarget` :`self` (`self.AbilitySystemComponent`) :`GameplayEffectClass` "/Game/Effects/GE_BossHit.GE_BossHit_C" :`Target` (`AbilitySystemBlueprintLibrary.GetAbilitySystemComponent` (`.HitActor` (`GameplayStatics.BreakHitResult` _outhit)))))

(fn `UserConstructionScript`)