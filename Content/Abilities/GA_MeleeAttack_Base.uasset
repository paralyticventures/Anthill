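; Base melee attack Gameplay Ability that plays a random attack montage using the avatar's equipped weapon from its WeaponsManagerComponent, ending if none exists.
; Montage-driven gameplay events for hit scan start and end toggle the weapon's hit detection.
; On start, the weapon receives a damage effect spec with SetByCaller magnitude under Data.Damage.
; Hit scan also stops when the ability ends, covering interrupted or cancelled montages.
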(event `HandleHitScanStart`
  ; Hit Scan Events
  (bind _equipped_weapon (`self.Equipped Weapon`)
    (:`then`
      (bind _returnvalue (`AbilitySystemBlueprintLibrary.AssignTagSetByCallerMagnitude` (`self.MakeOutgoingGameplayEffectSpec` (`self.DamageEffectClass`)) (struct :`TagName` "Data.Damage") (`self.DamageMagnitude`)))
      (`/Game/Weapons/BP_Weapon_Base.HitScanStart` _equipped_weapon _returnvalue))
    (:`else`)))

(event `HandleHitScanEnd`
  ; Hit Scan Events
  (bind _equipped_weapon (`self.Equipped Weapon`)
    (:`then`
      (`/Game/Weapons/BP_Weapon_Base.HitScanEnd` _equipped_weapon))
    (:`else`)))

(event `self.K2_ActivateAbility`
  (bind _attackmontage (`self.AttackMontage`))
  (bind _returnvalue (`Actor.GetComponentByClass` (`self.GetAvatarActorFromActorInfo`) "/Game/Weapons/WeaponsManagerComponent.WeaponsManagerComponent_C"))
  (`/Engine/EditorBlueprintResources/StandardMacros.IsValid` _returnvalue
    (:`Is Valid`
      (bind _equippedweapon (`/Game/Weapons/WeaponsManagerComponent.EquippedWeapon` _returnvalue)
        (:`then`
          (set `self.Equipped Weapon` _equippedweapon)
          (`AbilityTask_PlayMontageAndWait.CreatePlayMontageAndWaitProxy` "None" (`|GetArrayItem` _attackmontage (`KismetMathLibrary.RandomIntegerInRange` 0 (- (`KismetArrayLibrary.Array_Length` _attackmontage) 1))) 1.0 "None" true 1.0 0.0 true
            (:`then`
              (`AbilityTask_WaitGameplayEvent.WaitGameplayEvent` (struct :`TagName` "Event.HitScan.Start") null
                (:`then`
                  (`AbilityTask_WaitGameplayEvent.WaitGameplayEvent` (struct :`TagName` "Event.HitScan.End") null
                    (:`EventReceived`
                      (`self.HandleHitScanEnd`))))
                (:`EventReceived`
                  (`self.HandleHitScanStart`))))
            (:`OnCompleted`
              (`self.K2_EndAbility` :!label _label))
            (:`OnInterrupted`
              (goto _label))
            (:`OnCancelled`
              (goto _label))))
        (:`else`
          (`self.K2_EndAbility` :!label _label_2))))
    (:`Is Not Valid`
      (goto _label_2))))

(event `self.K2_OnEndAbility`
  (params (bWasCancelled :type Boolean))
  (`self.HandleHitScanEnd`))